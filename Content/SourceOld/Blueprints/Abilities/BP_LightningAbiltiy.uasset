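; Lightning ability actor whose movement mode gives the first-person player an aimed dash.
; While projecting, a camera-forward box trace moves the actor to preview the destination, pulled slightly back from the hit or max range.
; Casting puts the player in stasis, resizes the capsule and interpolates them there at constant speed without sweeping.
; On arrival it restores input mapping, releases stasis, destroys itself and applies forward exit velocity.
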(event EventBeginPlay
  (|CallParentFunction))

(event EventTick
  (params (DeltaSeconds :type Float%20%28single-precision%29))
  (bind _returnvalue (Game|GetPlayerController 0))
  (bind _firstpersonplayer (Variables|Default|GetFirstPersonPlayer))
  (bind _firstpersonplayer_2 (Variables|Default|GetFirstPersonPlayer))
  (bind _returnvalue_2 (PlayerController|LocalPlayerSubsystems|GetEnhancedInputLocalPlayerSubsystem _returnvalue))
  (if (Variables|Default|GetisInMovementMode)
    (if (Variables|Default|GetisProjecting)
      (CallFunction|ProjectDestination)
      (elif (Variables|Default|GetisDashing)
        (Transformation|SetActorLocation _firstpersonplayer (Math|Interpolation|VInterptoConstant (Transformation|GetActorLocation (Variables|Default|GetFirstPersonPlayer)) (Variables|Default|GetendLocation) DeltaSeconds (Variables|Default|GetDASH_SPEED)) false false)
        (if (Utilities|Operators|EqualEqual (Transformation|GetActorLocation _firstpersonplayer) (Variables|Default|GetendLocation) 0.01)
          (Input|RemoveMappingContext _returnvalue_2 "/Game/Source/Input/IMC_SpellReadied.IMC_SpellReadied" "(bIgnoreAllPressedKeysUntilRelease=True,bForceImmediately=False,bNotifyUserSettings=False)")
          (Input|AddMappingContext _returnvalue_2 "/Game/Source/Input/IMC_SpellControl.IMC_SpellControl" 0 "(bIgnoreAllPressedKeysUntilRelease=True,bForceImmediately=False,bNotifyUserSettings=False)")
          (Class|IMovementInhibitors|Unstasis(Message) (Variables|/Game/SourceOld/Blueprints/Entities/PlayerCharacter/BP_FirstPersonCharacter.BP_FirstPersonCharacter_C|GetBPC_Player_Movement _firstpersonplayer_2))
          (Class|IAbilityMessages|StopUsingAbility(Message) (Variables|/Game/SourceOld/Blueprints/Entities/PlayerCharacter/BP_FirstPersonCharacter.BP_FirstPersonCharacter_C|GetBPC_Ability_Deck _firstpersonplayer_2))
          (Actor|DestroyActor)
          (Variables|/Script/Engine.MovementComponent|SetVelocity (Variables|/Script/Engine.Character|GetCharacterMovement _firstpersonplayer_2) (* (Transformation|GetActorForwardVector _firstpersonplayer_2) (Variables|Default|GetdashEndSpeed))))))))

(fn ConstructionScript
  (|CallParentFunction))

(fn ActivateMovement
  (bind _returnvalue (Game|GetPlayerController 0))
  (bind _returnvalue_2 (PlayerController|LocalPlayerSubsystems|GetEnhancedInputLocalPlayerSubsystem _returnvalue))
  (Collision|SetActorEnableCollision false)
  (Input|RemoveMappingContext _returnvalue_2 "/Game/Source/Input/IMC_SpellControl.IMC_SpellControl" "(bIgnoreAllPressedKeysUntilRelease=True,bForceImmediately=False,bNotifyUserSettings=False)")
  (Input|AddMappingContext _returnvalue_2 "/Game/Source/Input/IMC_SpellReadied.IMC_SpellReadied" 0 "(bIgnoreAllPressedKeysUntilRelease=True,bForceImmediately=False,bNotifyUserSettings=False)")
  (Variables|Default|SetisProjecting true)
  (return true))

(fn ChannelMovement
  (return false))

(fn ProjectDestination
  (bind _firstpersonplayer (Variables|Default|GetFirstPersonPlayer))
  (bind _max_range (LocalVariables|GetMAX_RANGE))
  (bind _firstpersoncamera (Variables|/Game/SourceOld/Blueprints/Entities/PlayerCharacter/BP_FirstPersonCharacter.BP_FirstPersonCharacter_C|GetFirstPersonCamera _firstpersonplayer))
  (bind _firstpersoncamera_2 (Variables|/Game/SourceOld/Blueprints/Entities/PlayerCharacter/BP_FirstPersonCharacter.BP_FirstPersonCharacter_C|GetFirstPersonCamera _firstpersonplayer))
  (bind _returnvalue (Math|Vector|GetForwardVector _firstpersoncamera))
  (bind _returnvalue_2 (Transformation|GetWorldLocation _firstpersoncamera_2))
  (bind _returnvalue_3 (* _returnvalue 4e+01))
  (bind _returnvalue_4 (* _returnvalue _max_range))
  (bind _returnvalue_5 (+ _returnvalue_2 _returnvalue_4))
  (bind _outhit (Collision|BoxTraceByChannel _returnvalue_2 _returnvalue_5 "40.000000,40.000000,50.000000" "0, 0, 0" "TraceTypeQuery1" false 0 "None"))
  (if (.bblockinghit _outhit)
    (Transformation|SetActorLocation (- (.location _outhit) _returnvalue_3) false false)
    (else
      (Transformation|SetActorLocation (- _returnvalue_5 _returnvalue_3) false false))))

(fn CastSpell
  (bind _firstpersonplayer (Variables|Default|GetFirstPersonPlayer))
  (if (Variables|Default|GetisInMovementMode)
    (Variables|Default|SetisProjecting false)
    (Variables|Default|SetendLocation (Transformation|GetActorLocation))
    (Class|IMovementInhibitors|Stasis(Message) (Variables|/Game/SourceOld/Blueprints/Entities/PlayerCharacter/BP_FirstPersonCharacter.BP_FirstPersonCharacter_C|GetBPC_Player_Movement _firstpersonplayer))
    (Components|Capsule|SetCapsuleHalfHeight (Variables|/Script/Engine.Character|GetCapsuleComponent _firstpersonplayer) (Variables|Default|GetDASH_PLAYER_HALF_HEIGHT) true)
    (Variables|Default|SetisDashing true)))