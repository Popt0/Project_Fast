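; Player component that holds a capped deck of ability classes for the first-person character, starting with the lightning ability.
; Movement input spawns the current ability as an actor, activates it, then channels it while held if activation succeeded; cast input calls its spell.
; StopUsingAbility clears the active ability, advances the deck index with wraparound and re-enables movement casting.
; Adding to a full deck drops the oldest entry.
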(event Input|EnhancedActionEvents|EnhancedInputActionIA_MovementAbility
  (params (ActionValue :type Boolean) (ElapsedSeconds :type Float%20%28double-precision%29) (TriggeredSeconds :type Float%20%28double-precision%29) (InputAction :type Input%20Action%20Object%20Reference :default "/Game/Source/Input/Actions/IA_MovementAbility.IA_MovementAbility"))
  (bind _first_person_player (Variables|Default|GetFirst%20Person%20Player))
  (:Triggered
    ;[0.3939 0.8075 1] Channel Ability
    (if (Variables|Default|GetIsAbilityInUse)
      (Default|ChannelMovement (Variables|Default|GetActiveAbility))))
  (:Started
    ;[0.5925 1 0.6093] Start Ability
    (if (Variables|Default|GetcanCastMovement)
      (bind _returnvalue (Game|SpawnActorfromClass (Utilities|Array|Get(acopy) (Variables|Default|GetAbilities) (Variables|Default|GetCurrentActiveAbilityIndex)) (Math|Transform|MakeTransform (Transformation|GetActorLocation _first_person_player) (Transformation|GetActorRotation _first_person_player)) "Undefined" "MultiplyWithRoot" _first_person_player _first_person_player))
      (Utilities|IsValid _returnvalue
        (:Is%20Valid
          (bind _output_get (Variables|Default|SetActiveAbility _returnvalue))
          (bind _success (Default|ActivateMovement _output_get))
          (Variables|Default|SetIsAbilityInUse _success)
          (Variables|Default|SetcanCastMovement false))))))

(event Input|EnhancedActionEvents|EnhancedInputActionIA_Cast
  (params (ActionValue :type Boolean) (ElapsedSeconds :type Float%20%28double-precision%29) (TriggeredSeconds :type Float%20%28double-precision%29) (InputAction :type Input%20Action%20Object%20Reference :default "/Game/Source/Input/Actions/IA_Cast.IA_Cast"))
  (Default|CastSpell (Variables|Default|GetActiveAbility)))

(event EventBeginPlay
  (bind _asbp_first_person_character (Utilities|Casting|CastToBP_FirstPersonCharacter (Components|GetOwner)))
  (Variables|Default|SetFirst%20Person%20Player _asbp_first_person_character)
  (CallFunction|AddAbility "/Game/SourceOld/Blueprints/Abilities/BP_LightningAbiltiy.BP_LightningAbiltiy_C")
  (Input|AddMappingContext (PlayerController|LocalPlayerSubsystems|GetEnhancedInputLocalPlayerSubsystem (Game|GetPlayerController 0)) "/Game/Source/Input/IMC_SpellControl.IMC_SpellControl" 0 "(bIgnoreAllPressedKeysUntilRelease=True,bForceImmediately=False,bNotifyUserSettings=False)"))

(event EventTick
  (params (DeltaSeconds :type Float%20%28single-precision%29)))

(event EventStopUsingAbility
  (Variables|Default|SetIsAbilityInUse false)
  (Variables|Default|SetActiveAbility 0)
  (CallFunction|CycleAbility)
  (Variables|Default|SetcanCastMovement true))

(fn AddAbility
  (params (NewAbility :type BP%20Ability%20Class%20Reference))
  (if (< (Utilities|Array|Length (Variables|Default|GetAbilities)) (Variables|Default|GetMAX_ABILITIES))
    _
    (else
      (Utilities|Array|RemoveIndex (Variables|Default|GetAbilities))))
  (Utilities|Array|Add (Variables|Default|GetAbilities) NewAbility))

(fn CycleAbility
  (if (< (Variables|Default|GetCurrentActiveAbilityIndex) (- (Utilities|Array|Length (Variables|Default|GetAbilities)) 1))
    (Math|Integer|IncrementInt (Variables|Default|GetCurrentActiveAbilityIndex))
    (else
      (Variables|Default|SetCurrentActiveAbilityIndex 0))))