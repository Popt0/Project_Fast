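; BP_Ability is an ability Blueprint with stub hooks for movement and combat abilities, apparently meant as a base class.
; On BeginPlay it casts its owner to BP_FirstPersonCharacter and caches it as FirstPersonPlayer.
; Activate and Channel functions for movement and combat simply return true, with debug prints on the movement pair, and CastSpell is empty.
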(event EventBeginPlay
  (bind _asbp_first_person_character (Utilities|Casting|CastToBP_FirstPersonCharacter (Components|GetOwner)))
  (Variables|Default|SetFirstPersonPlayer _asbp_first_person_character))

(fn ConstructionScript)

(fn ActivateMovement
  (Development|PrintString "Start")
  (return true))

(fn ActivateCombat
  (return true))

(fn ChannelMovement
  (Development|PrintString "Channel")
  (return true))

(fn ChannelCombat
  (return true))

(fn CastSpell)