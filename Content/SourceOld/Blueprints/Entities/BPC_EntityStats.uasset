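; Actor component that tracks an entity's health in an EntityInfo struct and handles healing and damage.
; Damage subtracts from current health and destroys the owning actor when the result reaches zero or below.
; Heal adds health, but when the sum reaches max it stores the heal amount as current health instead of clamping.
; Each update rebuilds the struct, keeping name and max health while zeroing the last two fields.
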(event EventBeginPlay)

(event EventHeal
  (params (Health%20Healed :type Integer))
  (if (>= (+ Health%20Healed (.currenthealth (Variables|Default|GetentityInfo))) (.maxhealth (Variables|Default|GetentityInfo)))
    (Variables|Default|SetentityInfo (Utilities|Struct|MakeS_EntityData (.name (Variables|Default|GetentityInfo)) Health%20Healed (.maxhealth (Variables|Default|GetentityInfo)) 0 0.0))
    (else
      (Variables|Default|SetentityInfo (Utilities|Struct|MakeS_EntityData (.name (Variables|Default|GetentityInfo)) (+ Health%20Healed (.currenthealth (Variables|Default|GetentityInfo))) (.maxhealth (Variables|Default|GetentityInfo)) 0 0.0)))))

(event EventDamage
  (params (Damage%20Taken :type Integer))
  (if (<= (- (.currenthealth (Variables|Default|GetentityInfo)) Damage%20Taken) 0)
    (Actor|DestroyActor (Components|GetOwner))
    (else
      (Variables|Default|SetentityInfo (Utilities|Struct|MakeS_EntityData (.name (Variables|Default|GetentityInfo)) (- (.currenthealth (Variables|Default|GetentityInfo)) Damage%20Taken) (.maxhealth (Variables|Default|GetentityInfo)) 0 0.0)))))