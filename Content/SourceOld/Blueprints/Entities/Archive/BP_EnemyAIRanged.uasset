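; Ranged enemy AI logic for its owning BP_EnemyRanged, alternating between roaming and chasing the player, with a shooting event.
; SearchingRanged loops on AIMoveTo, picking random reachable points or, after a shot attempt flags LostPlayer, following the player pawn briefly.
; shootPlayer turns the enemy toward the player, spawns BP_FirstPersonProjectile from its ArrowGun, restarts searching and applies a cooldown.
; Nothing here calls shootPlayer, and the Searching function is empty.
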(event Custom|shootPlayer
  (if (Variables|Default|GetCanAttack)
    (Variables|Default|SetLostPlayer true)
    (bind _asbp_first_person_character (Utilities|Casting|CastToBP_FirstPersonCharacter (Game|Player|GetPlayerPawn 0)))
    (Variables|Default|SetLast%20Player%20Pos (Game|Player|GetPlayerPawn 0))
    (Transformation|SetActorRotation (Variables|Default|GetAs%20BP%20Enemy%20Ranged) (Math|Rotator|FindRelativeLookatRotation (Math|Conversions|ToTransform(Vector) (Transformation|GetActorLocation (Variables|Default|GetAs%20BP%20Enemy%20Ranged))) (Transformation|GetActorLocation _asbp_first_person_character)))
    (if (Variables|Default|GetCanAttack)
      (Game|SpawnActorfromClass "/Game/SourceOld/Blueprints/Entities/Archive/BP_FirstPersonProjectile.BP_FirstPersonProjectile_C" (Transformation|GetWorldTransform (Variables|/Game/SourceOld/Blueprints/Entities/Archive/BP_EnemyRanged.BP_EnemyRanged_C|GetArrowGun (Variables|Default|GetAs%20BP%20Enemy%20Ranged))) "Undefined" "MultiplyWithRoot" 0 0)
      (Variables|Default|SetCanAttack false)
      (CallFunction|SearchingRanged)
      (Utilities|FlowControl|Delay 1.0)
      (Variables|Default|SetCanAttack true))))

(event Custom|SearchingRanged
  ;[1 0.8945 0.1832] Searching
  (Utilities|FlowControl|Delay 0.5)
  (if (Variables|Default|GetLostPlayer)
    (AI|AIMoveTo (Variables|Default|GetAs%20BP%20Enemy%20Ranged) "0, 0, 0" (Variables|Default|GetLast%20Player%20Pos) 5.0 false
      (:then
        (Utilities|FlowControl|Delay 3.0)))
    (else
      (AI|AIMoveTo (Variables|Default|GetAs%20BP%20Enemy%20Ranged) (.RandomLocation (AI|Navigation|GetRandomReachablePointinRadius (Transformation|GetActorLocation (Variables|Default|GetAs%20BP%20Enemy%20Ranged)) 2.5e+03 0 0)) 0 5.0 false
        (:OnSuccess
          _))))
  (Variables|Default|SetLostPlayer false)
  (CallFunction|SearchingRanged))

(event EventBeginPlay
  (bind _asbp_enemy_ranged (Utilities|Casting|CastToBP_EnemyRanged (Components|GetOwner)))
  (Variables|Default|SetAs%20BP%20Enemy%20Ranged _asbp_enemy_ranged)
  (CallFunction|SearchingRanged))

(fn Searching)