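; Enemy AI component for a BP_Enemy owner that handles wandering and moving toward the player, with no attack logic.
; A self-restarting Searching event moves the enemy to random reachable points nearby, continuing only when a move succeeds.
; followPlayer flags the player as lost and targets the live pawn despite the LastPlayerPos name, then re-enters Searching, which repeats that move and clears the flag after a delay.
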(event Custom|followPlayer
  ;[1 1 1] Follow player
  (Variables|Default|SetLostPlayer true)
  (bind _output_get (Variables|Default|SetLastPlayerPos (Game|Player|GetPlayerPawn 0)))
  (AI|AIMoveTo (Variables|Default|GetBP_EnemyAI) "0, 0, 0" _output_get 5.0 false
    (:then
      (CallFunction|Searching))))

(event Custom|Searching
  ;[1 0.4843 0.1465] Searching
  (Utilities|FlowControl|Delay 0.5)
  (if (Variables|Default|GetLostPlayer)
    (AI|AIMoveTo (Variables|Default|GetBP_EnemyAI) "0, 0, 0" (Variables|Default|GetLastPlayerPos) 5.0 false
      (:then
        (Utilities|FlowControl|Delay 3.0)))
    (else
      (AI|AIMoveTo (Variables|Default|GetBP_EnemyAI) (.RandomLocation (AI|Navigation|GetRandomReachablePointinRadius (Transformation|GetActorLocation (Variables|Default|GetBP_EnemyAI)) 2.5e+03 0 0)) 0 5.0 false
        (:OnSuccess
          _))))
  (Variables|Default|SetLostPlayer false)
  (CallFunction|Searching))

(event EventBeginPlay
  (bind _asbp_enemy (Utilities|Casting|CastToBP_Enemy (Components|GetOwner)))
  (Variables|Default|SetBP_EnemyAI _asbp_enemy)
  (CallFunction|Searching))

(fn NewFunction)