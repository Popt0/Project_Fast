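; Base enemy Blueprint that detects the player, turns to aim and attacks on a cooldown, with UseAttack left as a placeholder.
; Each tick, a sphere trace finds the player, using separate alert and unalert radii, and a line trace checks line of sight.
; Once found, it rotates at constant speed toward LeadingShotRotation, fed by the projectile's default speed, and attacks when sight and cooldown allow.
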(event Custom|resetAttack
  (Variables|Combat|SetcanAttack true))

(event EventBeginPlay)

(event Collision|EventActorBeginOverlap
  (params (OtherActor :type Actor%20Object%20Reference)))

(event EventTick
  (params (DeltaSeconds :type Float%20%28single-precision%29))
  (CallFunction|DetectPlayer (Variables|Detection|GethasFoundPlayer))
  (if (Variables|Detection|GethasFoundPlayer)
    (Transformation|SetActorRotation (Class|KismetMathLibrary|RInterptoConstant (Transformation|GetActorRotation) (Utilities|LeadingShotRotation (.INITIAL_SPEED (Utilities|GetClassDefaults (Variables|Combat|GetATTACK_PROJECTILE)))) (Utilities|Time|GetWorldDeltaSeconds) (Variables|Default|GetTURN_SPEED)))
    (if (Variables|Detection|GethasPlayerLOS)
      (if (Variables|Combat|GetcanAttack)
        (Variables|Combat|SetcanAttack false)
        (CallFunction|UseAttack)
        (Utilities|Time|SetTimerbyEvent (delegate Custom|resetAttack) (Variables|Combat|GetATTACK_COOLDOWN))))))

(fn ConstructionScript)

(fn DetectPlayer
  (params (isAlert :type Boolean))
  (bind _returnvalue (Transformation|GetActorLocation))
  (bind (_outhits _returnvalue_2) (Collision|MultiSphereTraceForObjects _returnvalue _returnvalue (Math|Float|SelectFloat (Variables|Detection|GetALERT_DETECT_RADIUS) (Variables|Detection|GetUNALERT_DETECT_RADIUS) isAlert) (LocalVariables|GetdetectableObjectTypes) false 0 "ForOneFrame"))
  (if _returnvalue_2
    (bind (_array_element _array_index) (Utilities|Array|ForEachLoopwithBreak _outhits :!label _label)
      (:LoopBody
        (if (== (Game|Player|GetPlayerPawn 0) (.hitactor _array_element))
          (Variables|Detection|SethasFoundPlayer true)
          (bind _outhit (Collision|LineTraceByChannel (Transformation|GetActorLocation) (Transformation|GetActorLocation (Game|Player|GetPlayerPawn 0)) "TraceTypeQuery2" false 0 "ForOneFrame"))
          (if (== (Game|Player|GetPlayerPawn 0) (.hitactor _outhit))
            (Variables|Detection|SethasPlayerLOS true)
            (goto _label Break)
            (else
              (Variables|Detection|SethasPlayerLOS false)
              (goto _label Break)))
          (elif (== _array_index (Utilities|Array|LastIndex _outhits))
            (Variables|Detection|SethasFoundPlayer false)
            (Variables|Detection|SethasPlayerLOS false))))
      (:Completed
        (return (Variables|Detection|GethasFoundPlayer))))
    (else
      (Variables|Detection|SethasFoundPlayer false))))

(fn UseAttack
  (Development|PrintString "Add Attack Code Here"))