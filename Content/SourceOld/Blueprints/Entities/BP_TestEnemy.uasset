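; BP_TestEnemy is a test enemy actor whose only working behavior is a projectile attack.
; UseAttack spawns the configured projectile class at a forward offset from the actor, copying its rotation and scale.
; Nothing in this file calls the attack: the default events are disabled, the Cube sleep event is empty, and construction only runs the parent script.
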(event OnComponentSleep(Cube)
  (params (SleepingComponent :type Primitive%20Component%20Object%20Reference) (BoneName :type Name :default "None")))

(event EventBeginPlay
  (|CallParentFunction) ; This node is disabled and will not be called.\nDrag off pins to build functionality.
)

(event Collision|EventActorBeginOverlap
  (params (OtherActor :type Actor%20Object%20Reference))
  (|CallParentFunction OtherActor) ; This node is disabled and will not be called.\nDrag off pins to build functionality.
)

(event EventTick
  (params (DeltaSeconds :type Float%20%28single-precision%29))
  (|CallParentFunction DeltaSeconds) ; This node is disabled and will not be called.\nDrag off pins to build functionality.
)

(fn ConstructionScript
  (|CallParentFunction))

(fn UseAttack
  (bind _returnvalue (Transformation|GetActorTransform))
  (Game|SpawnActorfromClass (Variables|Default|GetATTACK_PROJECTILE) (Math|Transform|MakeTransform (+ (* (Transformation|GetActorForwardVector) (LocalVariables|GetPROJECTILE_OFFSET)) (.location _returnvalue)) (.rotation _returnvalue) (.scale _returnvalue)) "Undefined" "MultiplyWithRoot" 0 0)
  (return))