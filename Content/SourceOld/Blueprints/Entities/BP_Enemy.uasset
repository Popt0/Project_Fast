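; BP_Enemy is an enemy that turns to face the player and fires projectiles once it has found them.
; Each Tick branches on BPCPlayerDetection's HasFoundPlayer flag, running either the empty idle handler or the attack logic.
; The attack logic snaps rotation toward player pawn 0 and, when CanAttack allows, spawns a BP_Projectile just ahead of the enemy.
; A timer set by function name re-enables CanAttack after the cooldown.
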(event EventBeginPlay)

(event EventTick
  (params (DeltaSeconds :type Float%20%28single-precision%29))
  (if (Variables|/Game/SourceOld/Blueprints/Entities/BPC_PlayerDetection.BPC_PlayerDetection_C|GethasFoundPlayer (Variables|Default|GetBPC_PlayerDetection))
    (CallFunction|PlayerFoundEvents)
    (else
      (CallFunction|IdleEvents))))

(fn ConstructionScript)

(fn IdleEvents)

(fn PlayerFoundEvents
  (Transformation|SetActorRotation (Math|Rotator|FindLookatRotation (Transformation|GetActorLocation) (Transformation|GetActorLocation (Game|Player|GetPlayerPawn 0))))
  (if (Variables|Default|GetcanAttack)
    (CallFunction|UseAttack)
    (Variables|Default|SetcanAttack false)
    (Utilities|Time|SetTimerbyFunctionName 0 "resetAttackCooldown" (Variables|Default|GetATTACK_COOLDOWN))))

(fn ResetAttackCooldown
  (Variables|Default|SetcanAttack true))

(fn UseAttack
  (bind _returnvalue (Transformation|GetActorTransform))
  (Game|SpawnActorfromClass "/Game/SourceOld/Blueprints/Entities/BP_Projectile.BP_Projectile_C" (Math|Transform|MakeTransform (+ (* (Transformation|GetActorForwardVector) 5e+01) (.location _returnvalue)) (.rotation _returnvalue) (.scale _returnvalue)) "Undefined" "MultiplyWithRoot" 0 0))