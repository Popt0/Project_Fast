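; Player character component that tracks health stats and handles healing, damage and death.
; On BeginPlay it loads the PlayerCharacter row from DT_Entities and creates the WB_HUD health bar.
; Heal updates the HUD, but on reaching max sets health to the healed amount instead of the maximum.
; Damage destroys the owner at zero, otherwise only prints health; both events rebuild the struct, zeroing its last two fields.
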(event EventBeginPlay
  (bind _returnvalue (Utilities|GetDataTableRow "/Game/SourceOld/Blueprints/Entities/DT_Entities.DT_Entities" "PlayerCharacter")
    (:then
      (Variables|Default|SetplayerStats _returnvalue)
      (bind _returnvalue_2 (UserInterface|CreateWidget "/Game/SourceOld/Blueprints/UI/HUD/WB_HUD.WB_HUD_C" (Game|GetPlayerController 0)))
      (bind _output_get (Variables|Default|SetplayerHud _returnvalue_2))
      (Default|UpdateHealthBar _output_get (.currenthealth (Variables|Default|GetplayerStats)))
      (UserInterface|Viewport|AddtoViewport _output_get 0))))

(event EventHeal
  (params (Health%20Healed :type Integer))
  (if (>= (+ Health%20Healed (.currenthealth (Variables|Default|GetplayerStats))) (.maxhealth (Variables|Default|GetplayerStats)))
    (Variables|Default|SetplayerStats (Utilities|Struct|MakeS_EntityData (.name (Variables|Default|GetplayerStats)) Health%20Healed (.maxhealth (Variables|Default|GetplayerStats)) 0 0.0))
    (else
      (Variables|Default|SetplayerStats (Utilities|Struct|MakeS_EntityData (.name (Variables|Default|GetplayerStats)) (+ Health%20Healed (.currenthealth (Variables|Default|GetplayerStats))) (.maxhealth (Variables|Default|GetplayerStats)) 0 0.0))))
  (Default|UpdateHealthBar (Variables|Default|GetplayerHud) (.currenthealth (Variables|Default|GetplayerStats))))

(event EventDamage
  (params (Damage%20Taken :type Integer))
  (if (<= (- (.currenthealth (Variables|Default|GetplayerStats)) Damage%20Taken) 0)
    (Actor|DestroyActor (Components|GetOwner))
    (else
      (bind _output_get (Variables|Default|SetplayerStats (Utilities|Struct|MakeS_EntityData (.name (Variables|Default|GetplayerStats)) (- (.currenthealth (Variables|Default|GetplayerStats)) Damage%20Taken) (.maxhealth (Variables|Default|GetplayerStats)) 0 0.0)))
      (Development|PrintString (Utilities|String|ToString(Integer) (.currenthealth _output_get))))))