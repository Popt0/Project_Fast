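; Actor component that detects when the player's pawn is near its owning entity and exposes the result as HasFoundPlayer.
; Each tick it runs a zero-length multi-sphere object trace at the owner's location, drawn for debugging, and searches the hits for the player.
; The radius switches between alert and unalert values based on detection, but only when the trace hits something; an empty trace just clears the flag.
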(event EventBeginPlay
  (Variables|Default|SetcurrentDetectRadius (Variables|Default|GetUNALERT_DETECT_RADIUS)))

(event EventTick
  (params (DeltaSeconds :type Float%20%28single-precision%29))
  (CallFunction|DetectPlayer))

(fn DetectPlayer
  (bind _returnvalue (Components|GetOwner))
  (bind _returnvalue_2 (Transformation|GetActorLocation _returnvalue))
  (bind (_outhits _returnvalue_3) (Collision|MultiSphereTraceForObjects _returnvalue_2 _returnvalue_2 (Variables|Default|GetcurrentDetectRadius) (LocalVariables|GetdetectedObjectTypes) false 0 "ForOneFrame"))
  (if _returnvalue_3
    (bind (_array_element _array_index) (Utilities|Array|ForEachLoopwithBreak _outhits :!label _label)
      (:LoopBody
        (if (== (Game|Player|GetPlayerPawn 0) (.hitactor _array_element))
          (Variables|Default|SethasFoundPlayer true)
          (goto _label Break)
          (elif (== _array_index (Utilities|Array|LastIndex _outhits))
            (Variables|Default|SethasFoundPlayer false))))
      (:Completed
        (Variables|Default|SetcurrentDetectRadius (Math|Float|SelectFloat (Variables|Default|GetALERT_DETECT_RAIDUS) (Variables|Default|GetUNALERT_DETECT_RADIUS) (Variables|Default|GethasFoundPlayer)))))
    (else
      (Variables|Default|SethasFoundPlayer false))))