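; BP_Projectile is a projectile actor that damages the player on contact.
; BeginPlay copies its speed and gravity-scale variables onto the ProjectileMovement component.
; On Hit, if the other actor is the player pawn, it casts to BP_FirstPersonCharacter and calls DamageMessage on BPCPlayerStats with a fixed amount.
; It destroys itself after damaging the player or hitting anything else.
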(event EventBeginPlay
  (bind _projectilemovement (Variables|MyProjectile|GetProjectileMovement))
  (Variables|/Script/Engine.ProjectileMovementComponent|SetInitialSpeed _projectilemovement (Variables|Default|GetINITIAL_SPEED))
  (Variables|/Script/Engine.ProjectileMovementComponent|SetMaxSpeed _projectilemovement (Variables|Default|GetMAX_SPEED))
  (Variables|/Script/Engine.ProjectileMovementComponent|SetProjectileGravityScale _projectilemovement (Variables|Default|GetGRAV_SCALE)))

(event Collision|EventHit
  (params (MyComp :type Primitive%20Component%20Object%20Reference) (Other :type Actor%20Object%20Reference) (OtherComp :type Primitive%20Component%20Object%20Reference) (bSelfMoved :type Boolean) (HitLocation :type Vector :default "0, 0, 0") (HitNormal :type Vector :default "0, 0, 0") (NormalImpulse :type Vector :default "0, 0, 0") (Hit :type Hit%20Result%20Structure%20%28by%20ref%29))
  (if (== Other (Game|Player|GetPlayerPawn 0))
    (bind _asbp_first_person_character (Utilities|Casting|CastToBP_FirstPersonCharacter (Game|GetPlayerCharacter 0)))
    (Class|IHealthModifiers|Damage(Message) (Variables|/Game/SourceOld/Blueprints/Entities/PlayerCharacter/BP_FirstPersonCharacter.BP_FirstPersonCharacter_C|GetBPC_PlayerStats _asbp_first_person_character) 1))
  (Actor|DestroyActor))

(fn ConstructionScript)